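; BP_BaseCharacter2 is a development character Blueprint that prototypes mouse-aimed shooting with a debug line only.
; On Shoot, it intersects a line from the BP_CameraManager camera through the deprojected cursor with an X-normal plane at the actor's location, constraining aim to the YZ plane.
; It draws a short, persistent red line from the actor toward that point, with no projectile or damage logic.
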(event `InputAction|Shoot`
  (params (Key :type "Key Structure"))
  (bind _returnvalue (`self.K2_GetActorLocation`))
  (bind (_worldlocation _worlddirection) (`PlayerController.DeprojectMousePositionToWorld` (`GameplayStatics.GetPlayerController` 0)))
  (:`Pressed`
    (bind _returnvalue_2 (`GameplayStatics.GetActorOfClass` "/Game/Blueprints/Camera/BP_CameraManager.BP_CameraManager_C"))
    (`KismetSystemLibrary.DrawDebugLine` _returnvalue (+ _returnvalue (* (`KismetMathLibrary.GetDirectionUnitVector` _returnvalue (`.Intersection` (`KismetMathLibrary.LinePlaneIntersection_OriginNormal` (`SceneComponent.K2_GetComponentLocation` (`self.GetComponentByClass` _returnvalue_2 "/Script/Engine.CameraComponent")) (+ _worldlocation (* _worlddirection 2000)) _returnvalue (1.0 0.0 0.0)))) 100)) (struct :`R` 1.0 :`A` 1.0) 10.0 2.0)))

(event `self.ReceiveBeginPlay`)

(fn `UserConstructionScript`)